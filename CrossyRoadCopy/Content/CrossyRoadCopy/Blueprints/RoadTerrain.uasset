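; RoadTerrain is a road piece for a Crossy Road-style game that spawns vehicles along itself.
; On BeginPlay it caches the Start and End component locations and randomly picks one side as the spawn point for its lifetime.
; A looping timer, with an interval randomized once at startup, spawns a vehicle at that point, rotated 90 degrees either way depending on the side.
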(event `self.ReceiveBeginPlay`
  (set `self.StartLocation` (`SceneComponent.K2_GetComponentLocation` (`self.Start`)))
  (set `self.EndLocation` (`SceneComponent.K2_GetComponentLocation` (`self.End`)))
  (set `self.StartingCarLocation` (`KismetMathLibrary.RandomBool`))
  (`KismetSystemLibrary.K2_SetTimerDelegate` (delegate `Spawn Vehicles`) (`KismetMathLibrary.RandomFloatInRange` 2.0 3.0) true))

(event `Spawn Vehicles`
  (if (`self.StartingCarLocation`)
    (`|SpawnActorFromClass` "/Game/CrossyRoadCopy/Blueprints/Vehicles.Vehicles_C" (`KismetMathLibrary.MakeTransform` (`self.StartLocation`) (struct :`Yaw` 90.0)) "Undefined" "OverrideRootScale" null 300.0 null)
    (else
      (`|SpawnActorFromClass` "/Game/CrossyRoadCopy/Blueprints/Vehicles.Vehicles_C" (`KismetMathLibrary.MakeTransform` (`self.EndLocation`) (struct :`Yaw` -90.0)) "Undefined" "OverrideRootScale" null 300.0 null))))

(fn `UserConstructionScript`)