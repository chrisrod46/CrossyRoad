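; CollisionGrass is a grass lane actor for a Crossy Road-style game that scatters TreeRockSpawner actors as it begins play.
; It derives a slot count from the distance between its Start and End components, then steps along world Y from Start.
; Each slot has a roughly 30% random chance to spawn an actor.
; The count divisor and step size differ slightly, so slots can run past End.
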(event `self.ReceiveBeginPlay`
  (bind (_startlocation_x _startlocation_y _startlocation_z) (`KismetMathLibrary.BreakVector` (`self.StartLocation`)))
  (set `self.StartLocation` (`SceneComponent.K2_GetComponentLocation` (`self.Start`)))
  (set `self.EndLocation` (`SceneComponent.K2_GetComponentLocation` (`self.End`)))
  (for _index (range (+ (`KismetMathLibrary.FTrunc` (/ (`KismetMathLibrary.Vector_Distance` (`self.StartLocation`) (`self.EndLocation`)) 85.0)) 1))
    (if (> (`KismetMathLibrary.RandomFloat`) 0.7)
      (`|SpawnActorFromClass` "/Game/CrossyRoadCopy/Blueprints/TreeRockSpawner.TreeRockSpawner_C" (`KismetMathLibrary.MakeTransform` (`KismetMathLibrary.MakeVector` _startlocation_x (+ (* _index 90) (`.Y` (`KismetMathLibrary.BreakVector3f` (`self.StartLocation`)))) _startlocation_z)) "Undefined" "OverrideRootScale" null null))))

(fn `UserConstructionScript`)