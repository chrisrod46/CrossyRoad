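; Water terrain strip for a Crossy Road style game that spawns floating logs and ends the game when the chicken touches it.
; BeginPlay caches the Start and End positions, randomly picks one as the spawn side, and starts a looping timer with a randomized interval.
; Each tick of that timer spawns a Logs actor rotated for its side and binds the overlap handler.
; The handler calls Gameover on BP_ThirdPerson_Chicken through a DoOnce.
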(event `self.ReceiveBeginPlay`
  (set `self.StartLocation` (`SceneComponent.K2_GetComponentLocation` (`self.Start`)))
  (set `self.EndLocation` (`SceneComponent.K2_GetComponentLocation` (`self.End`)))
  (set `self.StartingLogLocation` (`KismetMathLibrary.RandomBool`))
  (`KismetSystemLibrary.K2_SetTimerDelegate` (delegate `Spawn Logs`) (`KismetMathLibrary.RandomFloatInRange` 2.0 3.0) true))

(event `Spawn Logs`
  (if (`self.StartingLogLocation`)
    (`|SpawnActorFromClass` "/Game/CrossyRoadCopy/Blueprints/Logs.Logs_C" (`KismetMathLibrary.MakeTransform` (`self.StartLocation`) (struct :`Yaw` 90.0)) "Undefined" "OverrideRootScale" null null)
    (else
      (`|SpawnActorFromClass` "/Game/CrossyRoadCopy/Blueprints/Logs.Logs_C" (`KismetMathLibrary.MakeTransform` (`self.EndLocation`) (struct :`Yaw` -90.0)) "Undefined" "OverrideRootScale" null null)))
  (add `self.OnActorBeginOverlap` (delegate `OnActorBeginOverlap_Event_0`)))

(event `OnActorBeginOverlap_Event_0` :!signature `self.OnActorBeginOverlap`
  (params (OverlappedActor :type "Actor Object Reference") (OtherActor :type "Actor Object Reference"))
  (bind _asbp_third_person_chicken (cast `/Game/CrossyRoadCopy/Blueprints/BP_ThirdPerson_Chicken` OtherActor))
  (`/Engine/EditorBlueprintResources/StandardMacros.DoOnce` false
    (:`Completed`
      (`/Game/CrossyRoadCopy/Blueprints/BP_ThirdPerson_Chicken.Gameover` _asbp_third_person_chicken))))

(fn `UserConstructionScript`)