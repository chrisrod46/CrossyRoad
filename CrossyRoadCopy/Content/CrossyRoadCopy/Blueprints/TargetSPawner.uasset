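; TargetSPawner is a lane obstacle actor for a Crossy Road copy that picks its appearance at random.
; On BeginPlay a random roll keeps the default Vehicle mesh or swaps it to a police car, long log or train, with the log and train also setting their own Box extent.
; Every Tick it destroys itself once its Y position leaves the fixed lane bounds; the graphs contain no movement or spawning logic.
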(event `self.ReceiveTick`
  (params (DeltaSeconds :type "Float (single-precision)"))
  (bind (_returnvalue_x _returnvalue_y) (`KismetMathLibrary.BreakVector` (`self.K2_GetActorLocation` self)))
  ;[1 1 1] Target Will Despawn outside Lanes
  (if (not (`KismetMathLibrary.InRange_FloatFloat` _returnvalue_y -600.0 600.0))
    (`self.K2_DestroyActor`)))

(event `self.ReceiveBeginPlay`
  (switch `int` (`KismetMathLibrary.RandomIntegerInRange` 0 3)
    (:`1`
      (`StaticMeshComponent.SetStaticMesh` (`self.Vehicle`) "/Game/CrossyRoadCopy/CrossyAssests/police_car.police_car"))
    (:`2`
      (`StaticMeshComponent.SetStaticMesh` (`self.Vehicle`) "/Game/CrossyRoadCopy/CrossyAssests/long_log.long_log")
      (`BoxComponent.SetBoxExtent` (`self.Box`) (-1.0 0.5 0.75) true))
    (:`3`
      (`StaticMeshComponent.SetStaticMesh` (`self.Vehicle`) "/Game/CrossyRoadCopy/CrossyAssests/train.train")
      (`BoxComponent.SetBoxExtent` (`self.Box`) (-3.0 0.5 0.75) true))))

(fn `UserConstructionScript`)