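; Terrain spawner for a Crossy Road-style game that lays an endless strip of terrain rows along X.
; On BeginPlay it spawns one segment: opening grass rows, then random road, grass, water or offset track rows.
; A CollisionGrass row mid-segment acts as a trigger: its first overlap by the chicken character spawns another TerrainSpawner at the segment's end, chaining the level onward.
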(event `self.ReceiveBeginPlay`
  (bind (_spawnlocation_x _spawnlocation_y _spawnlocation_z) (`KismetMathLibrary.BreakVector` (`self.SpawnLocation`)))
  (bind (_returnvalue_x _returnvalue_y _returnvalue_z) (`KismetMathLibrary.BreakVector` (`SceneComponent.K2_GetComponentLocation` (`self.StaticMesh`))))
  (for _index (range 31)
    (set `self.SpawnLocation` (`KismetMathLibrary.MakeVector` (+ (* _index 80) _returnvalue_x) _returnvalue_y _returnvalue_z))
    (if (`KismetMathLibrary.InRange_IntInt` _index 0 2)
      (`|SpawnActorFromClass` "/Game/CrossyRoadCopy/Blueprints/GrassTerrain.GrassTerrain_C" (`KismetMathLibrary.MakeTransform` (`self.SpawnLocation`)) "Undefined" "OverrideRootScale" null null)
      (elif (== _index 15)
        (bind _returnvalue (`|SpawnActorFromClass` "/Game/CrossyRoadCopy/Blueprints/CollisionGrass.CollisionGrass_C" (`KismetMathLibrary.MakeTransform` (`self.SpawnLocation`)) "Undefined" "OverrideRootScale" null null))
        (add `self.OnActorBeginOverlap` _returnvalue (delegate `OnActorBeginOverlap_Event_0`))
        (else
          (switch `int` (`KismetMathLibrary.RandomInteger` 4)
            (:`0`
              (`|SpawnActorFromClass` "/Game/CrossyRoadCopy/Blueprints/RoadTerrain.RoadTerrain_C" (`KismetMathLibrary.MakeTransform` (`self.SpawnLocation`)) "Undefined" "OverrideRootScale" null null))
            (:`1`
              (`|SpawnActorFromClass` "/Game/CrossyRoadCopy/Blueprints/GrassTerrain.GrassTerrain_C" (`KismetMathLibrary.MakeTransform` (`self.SpawnLocation`)) "Undefined" "OverrideRootScale" null null))
            (:`2`
              (`|SpawnActorFromClass` "/Game/CrossyRoadCopy/Blueprints/WaterTerrain.WaterTerrain_C" (`KismetMathLibrary.MakeTransform` (`self.SpawnLocation`)) "Undefined" "OverrideRootScale" null null))
            (:`3`
              (bind _output_get (set `self.SpawnLocation` (`KismetMathLibrary.MakeVector` _spawnlocation_x (+ _spawnlocation_y -30.0) (+ _spawnlocation_z -20.0))))
              (`|SpawnActorFromClass` "/Game/CrossyRoadCopy/Blueprints/TrackTerrain.TrackTerrain_C" (`KismetMathLibrary.MakeTransform` _output_get) "Undefined" "OverrideRootScale" null null))))))))

(event `OnActorBeginOverlap_Event_0` :!signature `self.OnActorBeginOverlap`
  (params (OverlappedActor :type "Actor Object Reference") (OtherActor :type "Actor Object Reference"))
  (bind (_returnvalue_x _returnvalue_y _returnvalue_z) (`KismetMathLibrary.BreakVector` (`SceneComponent.K2_GetComponentLocation` (`self.StaticMesh`))))
  (cast `/Game/CrossyRoadCopy/Blueprints/BP_ThirdPerson_Chicken` OtherActor)
  (`/Engine/EditorBlueprintResources/StandardMacros.DoOnce` false
    (:`Completed`
      (bind _output_get (set `self.SpawnLocation` (`KismetMathLibrary.MakeVector` (+ _returnvalue_x 2480.0) _returnvalue_y _returnvalue_z)))
      (`|SpawnActorFromClass` "TerrainSpawner_C" (`KismetMathLibrary.MakeTransform` _output_get) "Undefined" "OverrideRootScale" null null))))

(fn `UserConstructionScript`)